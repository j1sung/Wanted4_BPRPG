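; BP_BearController is the AI controller for the bear monster, starting its behavior when it possesses a pawn.
; On possession it sets up the BB_Bear blackboard and runs the BT_Bear behavior tree.
; It then seeds blackboard keys with the pawn's current location as home, a fixed patrol wait time and an initial state enum.
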(event `self.ReceivePossess`
  (params (PossessedPawn :type "Pawn Object Reference"))
  (`|ExecutionSequence`
    (:`then_0`
      (`self.UseBlackboard` "/Game/BluePrints/Monster/AI/BB_Bear.BB_Bear"))
    (:`then_1`
      (`self.RunBehaviorTree` "/Game/BluePrints/Monster/AI/BT_Bear.BT_Bear"))
    (:`then_2`
      (`BlackboardComponent.SetValueAsVector` (`AIBlueprintHelperLibrary.GetBlackboard` null) (`self.HomeLocationKey`) (`self.K2_GetActorLocation` PossessedPawn))
      (`BlackboardComponent.SetValueAsFloat` (`AIBlueprintHelperLibrary.GetBlackboard` null) (`self.PatrolWaitTimeKey`) 3.0)
      (`BlackboardComponent.SetValueAsEnum` (`AIBlueprintHelperLibrary.GetBlackboard` null) (`self.StateKey`) 4))))

(fn `UserConstructionScript`)