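; BP_HPController is a health component that tracks current and maximum HP for its owning actor.
; BeginPlay fills HP to maximum, and UpdateMaxHp sets a new maximum and refills to it.
; ReceiveDamage ignores hits once HP is depleted, otherwise subtracts damage, clamps at zero and fires OnDead on death.
; Every applied hit also broadcasts OnHpChanged with current and max HP, while UpdateMaxHp broadcasts nothing.
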(event `self.ReceiveBeginPlay`
  ;[0.8906 0.6686 0.08674 0.5] 시작할 때 최대체력으로
  (set `self.HealthPower` (`self.MaxHealthPower`)))

(event `ReceiveDamage`
  (params (Damage :type "Float (double-precision)"))
  ;[0.7708 0.2788 0.3267 0.5] 데미지 처리 - 과정에서 죽음 이벤트도 발행
  (if (> (`self.HealthPower`) 0.0)
    (bind _output_get (set `self.HealthPower` (- (`self.HealthPower`) Damage)))
    (if (<= _output_get 0.0)
      (set `self.HealthPower` 0.0)
      (`self.OnDeadEvent`)
      ;; HP 계산 재료 내기
      (`self.OnHpChanged` (`self.HealthPower`) (`self.MaxHealthPower`))
      (else
        ;; HP 계산 재료 내기
        (`self.OnHpChanged` (`self.HealthPower`) (`self.MaxHealthPower`))))))

(event `UpdateMaxHp`
  (params (MaxHealthPower :type "Float (double-precision)"))
  (bind _output_get (set `self.MaxHealthPower` MaxHealthPower))
  (set `self.HealthPower` _output_get))