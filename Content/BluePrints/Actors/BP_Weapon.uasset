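; BP_Weapon is a collectible weapon actor that deals melee-style damage through a toggled hit collision.
; Overlapping its Sphere notifies actors implementing BPI_WeaponPickup, then disables the Sphere; an older BP_Character cast remains unused.
; AttackCollision starts disabled and is query-only between the attack check begin and end events.
; Each actor it begins overlapping receives Damage, always credited to player controller 0.
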(event `self.Sphere.OnComponentBeginOverlap`
  (params (OverlappedComponent :type "PrimitiveComponent Object Reference") (OtherActor :type "Actor Object Reference") (OtherComp :type "PrimitiveComponent Object Reference") (OtherBodyIndex :type Integer) (bFromSweep :type Boolean) (SweepResult :type "HitResult Structure (by ref)"))
  ;[0.9583 0.8266 0 0.5] 무기 습득 처리
  (bind _asbpi_weapon_pickup (cast `/Game/BluePrints/Character/BPI_WeaponPickup` OtherActor))
  (`/Game/BluePrints/Character/BPI_WeaponPickup.OnWeaponCollected` _asbpi_weapon_pickup self)
  (`PrimitiveComponent.SetCollisionEnabled` (`self.Sphere`) "NoCollision"))

(event `self.ReceiveBeginPlay`
  ;[0.396 0.9531 0.3255 0.5] 시작시 끄기
  (`PrimitiveComponent.SetCollisionEnabled` (`self.AttackCollision`) "NoCollision"))

(event `OnAttackCheckBegin`
  ;[1 0.2539 0.2921 0.5] 공격 판정 시작
  (`PrimitiveComponent.SetCollisionEnabled` (`self.AttackCollision`) "QueryOnly"))

(event `OnAttackCheckEnd`
  ;[1 0.2214 0.2754 0.5] 공격 판정 종료
  (`PrimitiveComponent.SetCollisionEnabled` (`self.AttackCollision`) "NoCollision"))

(event `self.AttackCollision.OnComponentBeginOverlap`
  (params (OverlappedComponent :type "PrimitiveComponent Object Reference") (OtherActor :type "Actor Object Reference") (OtherComp :type "PrimitiveComponent Object Reference") (OtherBodyIndex :type Integer) (bFromSweep :type Boolean) (SweepResult :type "HitResult Structure (by ref)"))
  ;[0.15 0.687 0.15 0.5] 데미지 전달
  (`GameplayStatics.ApplyDamage` OtherActor (`self.Damage`) (`GameplayStatics.GetPlayerController` 0) self))

(fn `UserConstructionScript`)