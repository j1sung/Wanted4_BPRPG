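; BP_MonsterSpawner spawns monsters at its attached actors once the game starts, targeting the GameMode's kill target.
; On BeginPlay it gathers attached actors as spawn points, reads TargetKills from BP_GameMode and binds to OnGameStart.
; After a start delay, a self-rearming short timer spawns MonsterClass at random points, retrying failed spawns.
; Spawning stops when either the live monster count or SpawnCount reaches the target.
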(event `self.ReceiveBeginPlay`
  ;[0.987 0.1454 0.4293 0.5] 몬스터 시작 설정
  (bind _output_get (set `self.SpawnPoints` (`self.GetAttachedActors` true)))
  (if (> (`KismetArrayLibrary.Array_Length` _output_get) 0)
    (bind _asbp_game_mode (cast `/Game/BluePrints/Character/BP_GameMode` (`GameplayStatics.GetGameMode`)))
    (add `/Game/BluePrints/Character/BP_GameMode.OnGameStart` _asbp_game_mode (delegate `OnGameStart`))
    (set `self.TargetSpawnCount` (`/Game/BluePrints/Character/BP_GameMode.TargetKills` _asbp_game_mode))))

(event `OnGameStart`
  ;[0.987 0.1454 0.4293 0.5] 몬스터 시작 설정
  ;; 처음 스폰 시작 딜레이 3초
  (`KismetSystemLibrary.Delay` (`self.GameStartWaitTime`))
  (`self.StartSpawning`))

(event `StartSpawning`
  ;[0.8333 0.6567 0.3524 0.5] 몬스터 스폰
  ;; 빠르려면 Delay로 하거나
  (`KismetSystemLibrary.K2_SetTimerDelegate` (delegate `SpawnMonster`) 0.1) ; Time을 너무 낮추면 비동기 잘 안먹음
)

(event `SpawnMonster`
  ;[0.8333 0.6567 0.3524 0.5] 몬스터 스폰
  (bind _outactors (`GameplayStatics.GetAllActorsOfClass` (`self.MonsterClass`)))
  (if (< (`KismetArrayLibrary.Array_Length` _outactors) (`self.TargetSpawnCount`))
    (bind _returnvalue (`|SpawnActorFromClass` (`self.MonsterClass`) (`self.GetTransform` (`KismetArrayLibrary.Array_Random` (`self.SpawnPoints`))) "AdjustIfPossibleButAlwaysSpawn" "MultiplyWithRoot" null null))
    (`/Engine/EditorBlueprintResources/StandardMacros.IsValid` _returnvalue ; 생성 실패 시, 다시 스폰
      (:`Is Valid`
        (bind _result (`/Engine/EditorBlueprintResources/StandardMacros.IncrementInt` (`self.SpawnCount`))
          (:`  `
            (if (< _result (`self.TargetSpawnCount`))
              (`self.StartSpawning`)))))
      (:`Is Not Valid`
        (`self.StartSpawning`)))))

(fn `UserConstructionScript`)